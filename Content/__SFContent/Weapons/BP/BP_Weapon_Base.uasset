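; Base weapon actor that characters pick up, attaching it to their mesh and updating their animation, with a hover widget for interaction.
; Fire stores simulated projectile structs instead of spawning actors.
; Tick applies gravity drop, moves each by its unscaled per-frame velocity and line-traces the step for flat damage, never removing entries.
; Drop and velocity are adjustable at runtime, with debug traces and prints.
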(event Custom|Fire
  (bind _weapon_mesh (Variables|Default|GetWeapon%20Mesh))
  (bind _returnvalue (Transformation|GetSocketTransform _weapon_mesh "Base_Muzzle" "RTS_World"))
  (Utilities|Array|Add (Variables|Default|GetProjectiles) (Utilities|Struct|MakeS_ProjectileSim (.location _returnvalue) (Variables|Default|GetDrop) (* (Math|Vector|GetForwardVector (.rotation _returnvalue)) (Variables|Default|GetVelocity)) false 0)))

(event Custom|Change%20Drop
  (params (Delta%20Drop :type Float%20%28double-precision%29))
  (bind _output_get (Variables|Default|SetDrop (+ Delta%20Drop (Variables|Default|GetDrop))))
  (Development|PrintString (Utilities|String|ToString(Text) (Utilities|Text|FormatText "Drop = {a}" _output_get)) true true "(R=1.000000,G=0.000000,B=0.028928,A=1.000000)" 8.0))

(event Custom|Change%20Velocity
  (params (Delta%20Velocity :type Float%20%28double-precision%29))
  (bind _output_get (Variables|Default|SetVelocity (+ Delta%20Velocity (Variables|Default|GetVelocity))))
  (Development|PrintString (Utilities|String|ToString(Text) (Utilities|Text|FormatText "Velocity = {a}" _output_get)) true true "(R=0.000000,G=0.002356,B=1.000000,A=1.000000)" 8.0))

(event EventBeginPlay
  (Utilities|IsValid (Variables|Default|GetWeapon%20Mesh)))

(event EventTick
  (params (DeltaSeconds :type Float%20%28single-precision%29))
  (CallFunction|FunctUpdateBullets DeltaSeconds))

(event EventBPIFHoverInteraction
  (params (Hovering? :type Boolean))
  (bind _widget (Variables|Default|GetWidget))
  ;[0.15 0.15 0.15 0.5] Interacting
  (if Hovering?
    (bind _aswb_interact (Utilities|Casting|CastToWB_Interact (UserInterface|GetWidget (Variables|Default|GetWidget))))
    (Default|UpdateInfo _aswb_interact self)
    (Rendering|SetVisibility _widget true false)
    (else
      (Rendering|SetVisibility _widget false false))))

(event EventBPIInteract
  (params (Character%20Interacting :type Character%20Base%20Object%20Reference))
  (bind _mesh (Variables|/Script/Engine.Character|GetMesh Character%20Interacting))
  ;[0.15 0.15 0.15 0.5] Interacting
  (Physics|SetSimulatePhysics (Variables|Default|GetWeapon%20Mesh) false)
  (Collision|SetActorEnableCollision false) ; wierd shit with character movement happens if we dont do this for some reason
  (bind _asbp_char_base_2 (Utilities|Casting|CastToBP_Char_Base2 Character%20Interacting))
  (Variables|/Game/__SFContent/Characters/Blueprints/BP_Char_Base2.BP_Char_Base2_C|SetCurrent%20Weapon _asbp_char_base_2 self)
  (Transformation|AttachComponentToComponent _mesh (Variables|Default|GetSocket%20Attach) "SnapToTarget" "SnapToTarget" "SnapToTarget" true)
  (bind _asabp_skmmannequin (Utilities|Casting|CastToABP_SKMMannequin (Components|SkeletalMesh|GetAnimInstance _mesh)))
  (Default|UpdateAnimDT _asabp_skmmannequin (Utilities|String|StringToName (Utilities|String|ToString(Text) (Variables|Default|GetWeapon%20Name)))))

(fn ConstructionScript)

(fn FunctUpdateBullets
  (params (Delta%20Seconds :type Float%20%28single-precision%29))
  (bind _projectiles (Variables|Default|GetProjectiles))
  (for _index (range 0 (Utilities|Array|Length (Variables|Default|GetProjectiles)))
    (if (Utilities|Array|IsValidIndex _projectiles _index)
      (LocalVariables|SetNew%20Location (+ (.Location (Utilities|Struct|BreakS_ProjectileSim (Utilities|Array|Get(acopy) _projectiles _index))) (CallFunction|FunctCalculateDrop (.Velocity (Utilities|Struct|BreakS_ProjectileSim (Utilities|Array|Get(acopy) _projectiles _index))) (.GravityDrop (Utilities|Struct|BreakS_ProjectileSim (Utilities|Array|Get(acopy) _projectiles _index))) Delta%20Seconds)))
      (LocalVariables|SetNew%20Velocity (CallFunction|FunctCalculateDrop (.Velocity (Utilities|Struct|BreakS_ProjectileSim (Utilities|Array|Get(acopy) _projectiles _index))) (.GravityDrop (Utilities|Struct|BreakS_ProjectileSim (Utilities|Array|Get(acopy) _projectiles _index))) Delta%20Seconds))
      (bind _outhit (Collision|LineTraceByChannel (.Location (Utilities|Struct|BreakS_ProjectileSim (Utilities|Array|Get(acopy) _projectiles _index))) (+ (.Location (Utilities|Struct|BreakS_ProjectileSim (Utilities|Array|Get(acopy) _projectiles _index))) (CallFunction|FunctCalculateDrop (.Velocity (Utilities|Struct|BreakS_ProjectileSim (Utilities|Array|Get(acopy) _projectiles _index))) (.GravityDrop (Utilities|Struct|BreakS_ProjectileSim (Utilities|Array|Get(acopy) _projectiles _index))) Delta%20Seconds)) "TraceTypeQuery1" false 0 "Persistent" false))
      (Utilities|Struct|SetmembersinS_ProjectileSim (Utilities|Array|Get(acopy) _projectiles _index) (LocalVariables|GetNew%20Location) (LocalVariables|GetNew%20Velocity))
      (Game|Damage|ApplyDamage (.HitActor (Collision|BreakHitResult _outhit)) 25.0 0 0)
      (Development|PrintString (Utilities|GetDisplayName (.HitActor (Collision|BreakHitResult _outhit)))))))

(fn FunctCalculateDrop
  (params (Velocity :type Vector) (Gravity :type Float%20%28double-precision%29) (Delta%20Seconds :type Float%20%28double-precision%29))
  (bind (_x _y _z) (Math|Vector|BreakVector Velocity))
  (return (Math|Vector|MakeVector _x _y (+ _z (* Gravity Delta%20Seconds)))))

(fn BPIFGetActionType
  (return "NewEnumerator0"))

(fn BPIFGetInteractObjectInfo
  (return (Variables|Default|GetWeapon%20Name)))

(fn BPIFGetInteractType
  (return "NewEnumerator0"))