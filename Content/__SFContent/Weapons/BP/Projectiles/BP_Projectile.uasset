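; BP_Projectile is a projectile actor that takes its mesh from a data table row and launches after a delay.
; On BeginPlay it looks up the row set in NewVar, async loads the projectile mesh and applies it to ProjectileMesh.
; Once the mesh is set, a six-second timer activates ProjectileMovement, prints a debug string and switches player 0's view to the projectile.
; Blocking-load and row-iteration nodes are left unconnected.
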(event Custom|Activate
  (Development|PrintString "Hello")
  (Components|Activation|Activate (Variables|Default|GetProjectileMovement) false)
  (Game|Player|SetViewTargetwithBlend (Game|GetPlayerController 0) self 0.0 "VTBlend_Linear" 0.0 false))

(event EventBeginPlay
  (bind _newvar (Variables|Default|GetNewVar))
  (bind (_datatable _rowname) (Utilities|Struct|BreakDataTableRowHandle _newvar))
  (bind _returnvalue (Utilities|GetDataTableRow _datatable _rowname)
    (:then
      (bind _object (Utilities|AsyncLoadAsset (.projectilemesh (.ProjectileClassificationData (Utilities|Struct|BreakProjectileData _returnvalue))))
        (:Completed
          (bind _asstatic_mesh (Utilities|Casting|CastToStaticMesh _object))
          (Components|StaticMesh|SetStaticMesh (Variables|Default|GetProjectile%20Mesh) _asstatic_mesh)
          (Utilities|Time|SetTimerbyEvent (delegate Custom|Activate) 6.0))))))

(event Collision|EventActorBeginOverlap
  (params (OtherActor :type Actor%20Object%20Reference)))

(event EventTick
  (params (DeltaSeconds :type Float%20%28single-precision%29)))

(fn ConstructionScript)