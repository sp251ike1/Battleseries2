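; Prototype rotary-barrel weapon that runs an automatic firing demo: after a start delay it spins up, fires for a timed burst, then winds down.
; A per-frame looping timer interpolates barrel speed, which drives barrel rotation and the WeaponFire audio pitch and triggers.
; Near full speed, a fire-rate timer sweeps the gun side to side, spawning muzzle flashes and simulated projectiles through the projectile pool subsystem.
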(event Custom|Update%20Barrel%20Rotation
  (bind _weapon_fire (Variables|Default|GetWeapon%20Fire))
  ;[0.15 0.15 0.15 0.5] Update Barrel Rotation
  (if (Variables|Default|GetisSpinningUp)
    (Class|AudioParameterControllerInterface|SetTriggerParameter _weapon_fire "SpinUp")
    (bind _new_barrel_speed (CallFunction|FunctUpdateBarrelSpeed 1.0 (Variables|Default|GetBarrel%20Acceleraion)))
    (Audio|Parameter|SetFloatParameter (Variables|Default|GetWeapon%20Fire) "SpinUp_Pitch" _new_barrel_speed :!class /Script/AudioExtensions.AudioParameterControllerInterface)
    (Variables|Default|SetCurrent%20Barrel%20Rotation (CallFunction|FunctCalculatedNewTransform (Variables|Default|GetCurrent%20Barrel%20Rotation) (Variables|Default|GetBarrel%20Speed) 8e+02))
    (if (>= (Variables|Default|GetBarrel%20Speed) 0.9)
      (if (not (Utilities|Time|IsValidTimerHandle (Variables|Default|GetTimer_Fire)))
        (bind _returnvalue (Utilities|Time|SetTimerbyEvent (EventDispatchers|CreateEvent :!event Custom|Fire) (Class|WeaponFunctions|GetFireRate 9e+02) true))
        (Variables|Default|SetTimer_Fire _returnvalue)
        (bind _returnvalue_2 (Utilities|Time|SetTimerbyEvent (EventDispatchers|CreateEvent :!event Custom|Shutdown) 2e+01))
        (Variables|Default|SetTimer%20ShutDown _returnvalue_2)))
    (else
      ;;[0.15 0.15 0.15 0.5] Wind Down
      (Class|AudioParameterControllerInterface|SetTriggerParameter _weapon_fire "StopFire")
      (bind _result (Math|Float|NegateFloat (Variables|Default|GetBarrel%20Acceleraion))
        (:%20%20
          (bind _new_barrel_speed_2 (CallFunction|FunctUpdateBarrelSpeed 0.0 _result))
          (Audio|Parameter|SetFloatParameter (Variables|Default|GetWeapon%20Fire) "SpinUp_Pitch" _new_barrel_speed_2 :!class /Script/AudioExtensions.AudioParameterControllerInterface)
          (if (<= _new_barrel_speed_2 0.0)
            (Class|AudioParameterControllerInterface|SetTriggerParameter (Variables|Default|GetWeapon%20Fire) "Spin Down")
            (Utilities|Time|ClearandInvalidateTimerbyHandle (Variables|Default|GetTimer_BarrelRotation))))))))

(event Custom|Fire
  (bind _skeletalmesh (Variables|Default|GetSkeletalMesh))
  ;[0.15 0.15 0.15 0.5] Fire
  (Variables|Default|SetisFiring true)
  (bind _output_get (Variables|Default|SetCurrent%20Gun%20Rotation (CallFunction|FunctCalculatedNewTransform (Variables|Default|GetCurrent%20Gun%20Rotation) (Variables|Default|GetGun%20Rotation%20Speed) 1.0)))
  (if (< _output_get -45.0)
    (Math|Float|NegateFloat (Variables|Default|GetGun%20Rotation%20Speed) :!label _label
      (:%20%20
        _))
    (elif (> _output_get 45.0)
      (goto _label)
      (else
        _)))
  (Class|AudioParameterControllerInterface|SetTriggerParameter (Variables|Default|GetWeapon%20Fire) "StartFire")
  (Effects|SpawnEmitterAttached "/Game/ST_Minigun/Particles/PS_50cal_Muzzle.PS_50cal_Muzzle" _skeletalmesh "Fire" "0, 0, 0" "0, 0, 0" "2.000000,2.000000,2.000000")
  (Class|WeaponFunctions|CreateSimProjectile "P_Sim1" (Transformation|GetSocketLocation _skeletalmesh "Fire") 5.2e+04 0.0 (Math|Vector|GetForwardVector (Transformation|GetSocketRotation _skeletalmesh "Fire")) (Subsystems|GetProjectilePoolSubsystem)))

(event Custom|Shutdown
  ;[0.15 0.15 0.15 0.5] Shutdown
  (Variables|Default|SetisSpinningUp false)
  (Utilities|Time|ClearandInvalidateTimerbyHandle (Variables|Default|GetTimer_Fire)))

(event EventBeginPlay
  (Utilities|FlowControl|Delay 6.0)
  (Variables|Default|SetisSpinningUp true)
  (bind _returnvalue (Utilities|Time|SetTimerbyEvent (EventDispatchers|CreateEvent :!event Custom|Update%20Barrel%20Rotation) (Utilities|Time|GetWorldDeltaSeconds) true))
  (Variables|Default|SetTimer_BarrelRotation _returnvalue)
  (Components|Activation|Activate (Variables|Default|GetWeapon%20Fire) false))

(fn ConstructionScript)

(fn FunctCalculatedNewTransform
  (params (Current%20Transform%20Float :type Float%20%28double-precision%29) (Speed :type Float%20%28double-precision%29) (Multiplier :type Float%20%28double-precision%29))
  (return (+ Current%20Transform%20Float (* Speed (Utilities|Time|GetWorldDeltaSeconds) Multiplier))))

(fn FunctUpdateBarrelSpeed
  (params (Target :type Float%20%28double-precision%29) (Acceleration :type Float%20%28double-precision%29))
  (bind _output_get (Variables|Default|SetBarrel%20Speed (Math|Interpolation|FInterpTo (Variables|Default|GetBarrel%20Speed) Target (Utilities|Time|GetWorldDeltaSeconds) Acceleration)))
  (return _output_get))