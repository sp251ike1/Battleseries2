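; Manager actor for a loadout preview, showing a vehicle through its own view.
; The spawn function creates a preview character below the world origin and a vehicle at its Scene component, then sets itself as the first player's view target.
; A second function forwards a seat index to the preview vehicle to apply that seat's loadout.
; Event graph events are empty, and the spring arm rotation logic is unwired.
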(event EventBeginPlay)

(event Collision|EventActorBeginOverlap
  (params (OtherActor :type Actor%20Object%20Reference)))

(event EventTick
  (params (DeltaSeconds :type Float%20%28single-precision%29)))

(fn ConstructionScript)

(fn FunctSpawnPreviewVehicle
  (bind _returnvalue (Game|SpawnActorfromClass "/Script/Battleseries2.Character_Base" (Math|Transform|MakeTransform "0.000000,0.000000,-500.000000" "0, 0, 0" "1.000000,1.000000,1.000000") "Undefined" "MultiplyWithRoot" 0 0))
  (Variables|Default|SetPreview%20Character _returnvalue)
  (bind _returnvalue_2 (Game|SpawnActorfromClass "/Game/__SFContent/Vehicles/BP/BP_Vehicle_Base2.BP_Vehicle_Base2_C" (Math|Transform|MakeTransform (Transformation|GetWorldLocation (Variables|Default|GetScene)) "0, 0, 0" "1.000000,1.000000,1.000000") "Undefined" "MultiplyWithRoot" 0 0))
  (Variables|Default|SetPreview%20Vehicle _returnvalue_2)
  (Game|Player|SetViewTargetwithBlend (Game|GetPlayerController 0) self 0.0 "VTBlend_Linear" 0.0 false))

(fn FunctApplySeatOptionWeapon
  (params (Seat%20Index :type Integer))
  (Class|VehicleBase|ApplyLoadouttoSeat (Variables|Default|GetPreview%20Vehicle) Seat%20Index))