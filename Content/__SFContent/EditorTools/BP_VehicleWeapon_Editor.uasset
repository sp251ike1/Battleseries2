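; BP_VehicleWeapon_Editor is an editor-tool actor meant to preview a vehicle weapon's mesh while attached to a BP_Vehicle_Editor.
; Its construction script casts the attach parent and passes that vehicle's VehicleID, with its own WeaponID, to FunctQuickPreviewWeapMesh.
; That function is currently empty: the loop that matches WeaponID and sets VehicleWeaponMesh is disconnected, so no mesh is applied.
; The event graph has no active logic.
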(event EventBeginPlay)

(event Collision|EventActorBeginOverlap
  (params (OtherActor :type Actor%20Object%20Reference)))

(event EventTick
  (params (DeltaSeconds :type Float%20%28single-precision%29)))

(fn ConstructionScript
  (bind _asbp_vehicle_editor (Utilities|Casting|CastToBP_Vehicle_Editor (Actor|GetAttachParentActor)))
  (CallFunction|FunctQuickPreviewWeapMesh (Variables|/Game/__SFContent/EditorTools/BP_Vehicle_Editor.BP_Vehicle_Editor_C|GetVehicleID _asbp_vehicle_editor) (Variables|Default|GetWeaponID)))

(fn FunctQuickPreviewWeapMesh
  (params (VehicleID :type Name) (WeaponID :type Name)))