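; Editor tool actor that previews a simple vehicle bone animation by sliding one named bone of a poseable mesh vertically.
; The construction script caches the bone's component-space X and Y and places it at StartZ.
; Each Tick lerps Z toward EndZ by a frame counter rather than delta time, printing the offset.
; When the counter reaches MaxFrames, Reset snaps the bone back to StartZ and the motion loops.
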(event Custom|Reset
  (bind _baseboneoffset (Variables|Default|GetBaseBoneOffset))
  (Class|PoseableMeshComponent|SetBoneLocationbyName (Variables|Default|GetPoseableMesh) (Variables|Default|GetBoneName) (Math|Vector|MakeVector (.x _baseboneoffset) (.y _baseboneoffset) (Variables|Default|GetStartZ)) "ComponentSpace")
  (Variables|Default|SetFrameCounter 1))

(event EventBeginPlay
  (CallFunction|Reset))

(event EventTick
  (params (DeltaSeconds :type Float%20%28single-precision%29))
  (if (< (Variables|Default|GetFrameCounter) (Variables|Default|GetMaxFrames))
    (bind _output_get (Variables|Default|SetCurrentZ (Math|Float|Lerp (Variables|Default|GetStartZ) (Variables|Default|GetEndZ) (/ (Math|Conversions|ToFloat(Integer) (Variables|Default|GetFrameCounter)) (Math|Conversions|ToFloat(Integer) (- (Variables|Default|GetMaxFrames) 1))))))
    (bind _output_get_2 (Variables|Default|SetBaseBoneOffset (Math|Vector|MakeVector (.x (Variables|Default|GetBaseBoneOffset)) (.y (Variables|Default|GetBaseBoneOffset)) _output_get)))
    (Class|PoseableMeshComponent|SetBoneLocationbyName (Variables|Default|GetPoseableMesh) (Variables|Default|GetBoneName) _output_get_2 "ComponentSpace")
    (Math|Integer|IncrementInt (Variables|Default|GetFrameCounter)
      (:%20%20
        (Development|PrintString (Utilities|String|ToString(Vector) _output_get_2))))
    (else
      (CallFunction|Reset))))

(fn ConstructionScript
  (bind _returnvalue (Class|PoseableMeshComponent|GetBoneLocationbyName (Variables|Default|GetPoseableMesh) (Variables|Default|GetBoneName) "ComponentSpace"))
  (bind _output_get (Variables|Default|SetBaseBoneOffset (Math|Vector|MakeVector (.x _returnvalue) (.y _returnvalue) (Variables|Default|GetStartZ))))
  (Class|PoseableMeshComponent|SetBoneLocationbyName (Variables|Default|GetPoseableMesh) (Variables|Default|GetBoneName) _output_get "ComponentSpace"))