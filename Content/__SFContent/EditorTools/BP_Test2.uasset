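; BP_Test2 is a test interactable actor that attaches the interacting character to itself.
; On BPIInteract it disables the character's collision, attaches it with keep-relative rules, and sets its relative transform to that of the BPTest component, printing that transform for debugging.
; The other interaction interface functions return a fixed enum entry or empty info, and the construction script is empty.
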(event EventBeginPlay)

(event Collision|EventActorBeginOverlap
  (params (OtherActor :type Actor%20Object%20Reference)))

(event EventTick
  (params (DeltaSeconds :type Float%20%28single-precision%29)))

(event EventBPIInteract
  (params (Character%20Interacting :type Character%20Base%20Object%20Reference))
  (bind _bp_test (Variables|Default|GetBP_Test))
  (bind _returnvalue (Transformation|GetRelativeTransform _bp_test))
  (Collision|SetActorEnableCollision Character%20Interacting false)
  (Transformation|AttachActorToActor Character%20Interacting self "None" "KeepRelative" "KeepRelative" "KeepRelative" true)
  (Transformation|SetActorRelativeTransform Character%20Interacting _returnvalue false false)
  (Development|PrintString (Utilities|String|ToString(Transform) _returnvalue)))

(fn ConstructionScript)

(fn BPIFGetActionType
  (return "NewEnumerator0"))

(fn BPIFGetInteractObjectInfo
  (return ""))

(fn BPIFGetInteractType
  (return "NewEnumerator0"))