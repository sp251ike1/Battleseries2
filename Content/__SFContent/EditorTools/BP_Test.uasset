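; BP_Test is an editor-tools test actor that implements an interaction interface but does nothing when interacted with.
; Its interface getters return fixed values: the first action and interact type enum entries and "TEST" as object info.
; Disconnected, never-run nodes hold experiments in disabling collision, snapping the interacting character to the actor, and attaching or detaching actors and components.
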(event EventBeginPlay)

(event Collision|EventActorBeginOverlap
  (params (OtherActor :type Actor%20Object%20Reference)))

(event EventTick
  (params (DeltaSeconds :type Float%20%28single-precision%29)))

(event EventBPIInteract
  (params (Character%20Interacting :type BP%20Char%20Base%202%20Object%20Reference)))

(fn ConstructionScript)

(fn BPIFGetActionType
  (return "NewEnumerator0"))

(fn BPIFGetInteractObjectInfo
  (return "TEST"))

(fn BPIFGetInteractType
  (return "NewEnumerator0"))