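; BP_Vehicle_Editor is an editor-tool actor that previews a vehicle and its seat layout from a data table row selected by VehicleID.
; The construction script blocking-loads the row's skeletal mesh, then indexes child-actor BP_Seat_Editors by SeatIndex, activating those below the row's seat count.
; BeginPlay also spawns an extra seat editor and, after a short delay, attaches it at a hardcoded offset.
; Older seat and weapon-preview logic remains in the construction script, disconnected.
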(event EventBeginPlay
  (bind _returnvalue (Game|SpawnActorfromClass "/Game/__SFContent/EditorTools/BP_Seat_Editor.BP_Seat_Editor_C" (Math|Transform|MakeTransform "0, 0, 0" "0, 0, 0" "1.000000,1.000000,1.000000") "AlwaysSpawn" "MultiplyWithRoot" 0 0))
  (Utilities|FlowControl|Delay 0.2)
  (Transformation|AttachActorToActor _returnvalue self "None" "KeepRelative" "KeepRelative" "KeepRelative" false)
  (Transformation|SetActorRelativeTransform _returnvalue (Math|Transform|MakeTransform "495.000000,-2.000000,297.000000" "0, 0, 0" "1.000000,1.000000,1.000000") false false))

(event Collision|EventActorBeginOverlap
  (params (OtherActor :type Actor%20Object%20Reference)))

(event EventTick
  (params (DeltaSeconds :type Float%20%28single-precision%29)))

(fn ConstructionScript
  (CallFunction|FunctLoadVehicleMeshinEditor)
  (CallFunction|FunctConfigureSeats))

(fn FunctLoadVehicleMeshinEditor
  (bind _returnvalue (Utilities|LoadAssetBlocking (Utilities|Struct|BreakVehicleData (CallFunction|FunctGetVehicleData))))
  (bind _asskeletal_mesh (Utilities|Casting|CastToSkeletalMesh _returnvalue))
  (Components|SkeletalMesh|SetSkeletalMeshAsset (Variables|Default|GetVehicle%20Mesh) _asskeletal_mesh))

(fn FunctGetVehicleData
  (bind _returnvalue (Utilities|GetDataTableRow (Variables|Default|GetVehicle%20DT) (Variables|Default|GetVehicleID))
    (:then
      (return _returnvalue))))

(fn FunctConfigureSeats
  (Utilities|FlowControl|Sequence
    (:then_0
      (bind _output_get (Variables|Default|Set#%20of%20Seats (Utilities|Array|Length (Utilities|Struct|BreakVehicleData (CallFunction|FunctGetVehicleData)))))
      (Development|PrintString (Utilities|String|ToString(Integer) _output_get)))
    (:then_1
      (for _array_element (Actor|GetComponentsByClass "/Script/Engine.ChildActorComponent")
        (bind _asbp_seat_editor (Utilities|Casting|CastToBP_Seat_Editor (Variables|/Script/Engine.ChildActorComponent|GetChildActor _array_element)))
        (bind _output_get_2 (LocalVariables|SetSeat _asbp_seat_editor))
        (bind _output_get_3 (LocalVariables|SetSeat%20Index (Variables|/Game/__SFContent/EditorTools/BP_Seat_Editor.BP_Seat_Editor_C|GetSeat%20Index _output_get_2)))
        (Utilities|Array|SetArrayElem (Variables|Default|GetEditorSeats) _output_get_3 _output_get_2)
        (if (< (LocalVariables|GetSeat%20Index) (Variables|Default|Get#%20of%20Seats))
          (Variables|/Game/__SFContent/EditorTools/BP_Seat_Editor.BP_Seat_Editor_C|SetisActive (LocalVariables|GetSeat) true)
          (else
            (Variables|/Game/__SFContent/EditorTools/BP_Seat_Editor.BP_Seat_Editor_C|SetisActive (LocalVariables|GetSeat) false)))))))