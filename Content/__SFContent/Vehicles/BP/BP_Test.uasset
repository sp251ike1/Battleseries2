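; BP_Test is a vehicle test Blueprint that adds a Chaos wheeled vehicle movement component on BeginPlay and holds prototype weapon-aiming helpers.
; The rangefinder line-traces on Visibility from zeroed placeholder origin and rotation with persistent debug drawing, storing the hit or trace end as TargetPoint.
; The aim function normalizes the vector from SocketLocation to TargetPoint.
; The muzzle transform function is an unwired stub, and nothing in the event graph calls these helpers.
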(event EventBeginPlay
  (bind _returnvalue (Game|AddComponentbyClass "/Script/ChaosVehicles.ChaosWheeledVehicleMovementComponent"))
  (Variables|Default|SetCWVM _returnvalue))

(fn ConstructionScript)

(fn FunctMuzzleTransform)

(fn FunctGetAimDirection
  (return (Math|Vector|Normalize (- (Variables|Default|GetTargetPoint) (Variables|Default|GetSocketLocation)))))

(fn FunctRangefinder
  (bind _outhit (Collision|LineTraceByChannel "0, 0, 0" (+ "" (* (Math|Rotator|GetRotationXVector "0, 0, 0") 5e+04)) "TraceTypeQuery1" true 0 "Persistent" false))
  (if (.bBlockingHit (Collision|BreakHitResult _outhit))
    (bind _output_get (Variables|Default|SetImpact%20Point (.ImpactPoint (Collision|BreakHitResult _outhit))))
    (Variables|Default|SetTargetPoint _output_get)
    (else
      (bind _output_get_2 (Variables|Default|SetTrace%20End (.TraceEnd (Collision|BreakHitResult _outhit))))
      (Variables|Default|SetTargetPoint _output_get_2))))