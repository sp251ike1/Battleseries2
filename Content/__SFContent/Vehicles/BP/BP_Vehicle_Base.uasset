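; Base vehicle Blueprint with multiple seats, an interface-driven interaction prompt shown on hover, and hover-style flight controls.
; On BeginPlay it sorts child-actor seats by index into SeatData and socket-attaches spring arms for remote-camera seats; a helper finds free seats for cycling.
; Throttle adds interpolated velocity along the up vector, easing to HoverPower at zero input, while pitch applies interpolated local rotation.
; Tick feeds constant yaw to ChaosWheeledVehicleMovement; the interact event is an empty stub.
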(event Custom|UpdateThrottle
  (params (AV :type Float%20%28double-precision%29))
  (bind _returnvalue (Utilities|Time|GetWorldDeltaSeconds))
  (bind _mesh (Variables|Character|GetMesh))
  (bind _rootcomponent (Variables|Transformation|GetRootComponent))
  (bind _returnvalue_2 (Math|Vector|GetUpVector _rootcomponent))
  (if (!= AV 0.0)
    (bind _output_get (Variables|Default|SetHover_velocity (Math|Interpolation|FInterpTo (Variables|Default|GetHover_velocity) (* AV (Variables|Default|GetMax%20thrust)) _returnvalue 2.0)))
    (Class|PrimitiveComponent|SetAllPhysicsLinearVelocity _mesh (* (* _returnvalue_2 _output_get) (* (Utilities|Time|GetWorldDeltaSeconds) 1e+02)) true)
    (else
      (bind _output_get_2 (Variables|Default|SetHover_velocity (Math|Interpolation|FInterpTo (Variables|Default|GetHover_velocity) (Variables|Default|GetHover%20Power) _returnvalue 4.0)))
      (Class|PrimitiveComponent|SetAllPhysicsLinearVelocity _mesh (* (* _returnvalue_2 _output_get_2) (* (Utilities|Time|GetWorldDeltaSeconds) 1e+02)) true))))

(event Custom|UpdatePitch
  (params (AV :type Float%20%28double-precision%29))
  (bind _output_get (Variables|Default|SetPitch%20Speed (Math|Interpolation|FInterpTo (Variables|Default|GetPitch%20Speed) (* AV (Variables|Default|GetMax%20Pitch%20Speed)) (Utilities|Time|GetWorldDeltaSeconds) 1.5)))
  (Transformation|AddActorLocalRotation (Math|Rotator|MakeRotator 0.0 _output_get 0.0) false true))

(event EventBeginPlay
  (CallFunction|FunctSetupSeats))

(event EventTick
  (params (DeltaSeconds :type Float%20%28single-precision%29))
  (Class|ChaosVehicleMovementComponent|SetYawInput (Variables|Default|GetChaosWheeledVehicleMovement) 1.0))

(event EventBPIFHoverInteraction
  (params (Hovering? :type Boolean))
  (bind _widget (Variables|Default|GetWidget))
  (if Hovering?
    (bind _aswb_interact (Utilities|Casting|CastToWB_Interact (UserInterface|GetWidget (Variables|Default|GetWidget))))
    (Default|UpdateInfo _aswb_interact self)
    (Rendering|SetVisibility _widget true false)
    (else
      (Rendering|SetVisibility _widget false false))))

(event EventBPIInteract
  (params (Character%20Interacting :type Character%20Base%20Object%20Reference))
  ;[0.15 0.15 0.15 0.5] called by characters entering vehicle
)

(fn ConstructionScript)

(fn FunctCycleThroughSeats
  (params (Character :type BP%20Char%20Base%20Object%20Reference))
  (bind _csi (Variables|/Game/__SFContent/Characters/Blueprints/BP_Char_Base.BP_Char_Base_C|GetCSI Character))
  (bind _index (Utilities|FlowControl|ForLoopwithBreak (Variables|/Game/__SFContent/Characters/Blueprints/BP_Char_Base.BP_Char_Base_C|GetNSI Character) (Utilities|Array|LastIndex (Variables|Default|GetSeat%20Data)) :!label _label)
    (:LoopBody
      (Utilities|IsValid (.CharacterOccupied? (Utilities|Struct|BreakStruct_Seats (Utilities|Array|Get(acopy) (Variables|Default|GetSeat%20Data) _index)))
        (:Is%20Not%20Valid
          (Variables|/Game/__SFContent/Characters/Blueprints/BP_Char_Base.BP_Char_Base_C|SetNSI Character _index)
          (Utilities|FlowControl|Sequence
            (:then_0
              (goto _label Break))
            (:then_1
              (return true))))))
    (:Completed
      (if (== (Variables|/Game/__SFContent/Characters/Blueprints/BP_Char_Base.BP_Char_Base_C|GetNSI Character) _csi)
        (bind _index_2 (Utilities|FlowControl|ForLoopwithBreak 0 (- _csi 1) :!label _label_2)
          (:LoopBody
            (Utilities|IsValid (Utilities|Struct|BreakStruct_Seats (Utilities|Array|Get(acopy) (Variables|Default|GetSeat%20Data) _index_2))
              (:Is%20Not%20Valid
                (Variables|/Game/__SFContent/Characters/Blueprints/BP_Char_Base.BP_Char_Base_C|SetNSI Character _index_2)
                (Utilities|FlowControl|Sequence
                  (:then_0
                    (return true))
                  (:then_1
                    (goto _label_2 Break))))))
          (:Completed
            (return false)))))))

(fn FunctSetupSeats
  (for _array_element (Actor|GetComponentsByClass "/Script/Engine.ChildActorComponent")
    (bind _asbp_seat_base (Utilities|Casting|CastToBP_Seat_Base (Variables|/Script/Engine.ChildActorComponent|GetChildActor _array_element)))
    (Utilities|Array|SetArrayElem (LocalVariables|GetSeat%20Array) (Variables|/Game/__SFContent/Vehicles/BP/BP_Seat_Base.BP_Seat_Base_C|GetSeat%20Index _asbp_seat_base) _asbp_seat_base))
  (for (_array_element_2 _array_index) (LocalVariables|GetSeat%20Array)
    (bind _structout (Utilities|Struct|SetmembersinStruct_Seats (Utilities|Array|Get(acopy) (Variables|Default|GetSeat%20Data) _array_index) _array_element_2))
    (switch Utilities|FlowControl|Switch|SwitchonEnum_CameraMgmt (.CameraMgmt (Utilities|Struct|BreakStruct_Seats _structout))
      (:NewEnumerator1
        (Transformation|AttachComponentToComponent (Variables|/Game/__SFContent/Vehicles/BP/BP_Seat_Base.BP_Seat_Base_C|GetSpringArm (.SeatPawn (Utilities|Struct|BreakStruct_Seats _structout))) (Variables|Transformation|GetRootComponent) (Utilities|String|StringToName (Utilities|String|ToString(Text) (Utilities|Text|FormatText "Seat{SeatIndex}" _array_index))) "SnapToTarget" "SnapToTarget" "SnapToTarget" true)))))

(fn BPIFGetActionType
  (return "NewEnumerator1"))

(fn BPIFGetInteractObjectInfo
  (return (Variables|Default|GetVehicle%20Name)))

(fn BPIFGetInteractType
  (return "NewEnumerator1"))

(fn BPIFReturnSeat
  (params (Seat%20Index :type Integer))
  (return (Utilities|Array|Get(acopy) (Variables|Default|GetSeat%20Data) Seat%20Index)))

(fn BPIFReturnVehicleWeapon
  (params (SeatIndex :type Integer))
  (return 0))